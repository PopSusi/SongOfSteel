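; Central controller for an orchestra-upkeep game's day flow, which initializes the game instance and day-track HUD on BeginPlay.
; It spawns a TransitionManager, shows an inherited-will letter on day zero, then chains Letters and SongSelect widgets through close events into spawning management.
; Separate dialogue logic picks a random event by priority tier, though the mid-tier call passes no pool.
; SetDialogue displays lines, reveals two choices and resolves finished scenes into the autosave.
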(event `self.ReceiveBeginPlay`
  (bind _returnvalue (`|CreateWidget` "/Game/UI/DayTrack.DayTrack_C"))
  (bind _output_get (set `self.DayTrackUI` _returnvalue))
  (`UserWidget.AddToPlayerScreen` _output_get 0)
  (bind _instance (`/Game/DataTypes/General/SaveAccess.Get Instance` _output_get))
  (bind _output_get_2 (set `self.Instance` _instance))
  (`/Game/Blueprints/Instance.Initialize Game` _instance)
  (`/Game/Blueprints/Instance.Initialize Game` _output_get_2)
  (`/Game/UI/DayTrack.Initialize` _output_get)
  (`self.SpawnTrans`))

(event `Assigns`
  (add `/Game/Blueprints/Instance.EventsInitialized` (`self.Instance`) (delegate `PickDialogue`)))

(event `PickDialogue`
  (bind _instance (`self.Instance`))
  (bind _highpriorityevents (`/Game/Blueprints/Instance.HighPriorityEvents` (`self.Instance`)))
  (if (`KismetArrayLibrary.Array_IsNotEmpty` _highpriorityevents)
    (`self.PickRandomEvent` _highpriorityevents)
    (elif (`KismetArrayLibrary.Array_IsNotEmpty` (`/Game/Blueprints/Instance.MidPriorityEvents` _instance))
      (`self.PickRandomEvent` _)
      (else
        (`self.PickRandomEvent` (`/Game/Blueprints/Instance.LowPriorityEvents` _instance)))))
  (`self.ClearUI`))

(event `DayOne`
  (bind _returnvalue (`|SpawnActorFromClass` "/Game/DataTypes/General/TransitionManager.TransitionManager_C" (`KismetMathLibrary.MakeTransform` (0.0 0.0 0.0)) "Undefined" "MultiplyWithRoot" null null :!label _label))
  (set `self.TransManage` _returnvalue)
  (if (== (`/Game/Blueprints/Instance.CurrentDay` (`self.Instance`)) 0)
    (bind _returnvalue_2 (`|CreateWidget` "/Game/UI/LetterSystem/BPW_ResLetter.BPW_ResLetter_C"))
    (bind _output_get (set `self.Tutorial` _returnvalue_2))
    (`UserWidget.AddToPlayerScreen` _output_get 0)
    (message `/Game/DataTypes/Events/Letters/LetterValueSet.SetValues` _output_get "My Will" "As I write this letter, I stare death in the face and yet I feel no fear. The fear that I previously let control my life has now left my body, and I will now tackle all of my sins shortly after finishing this letter. My Son, I grieve the thought of my orchestra falling with myself. So I have but one request, my son. I only ask for you to keep maintenance on the orchestra. You should be able to purchase everything you need at the local market. In the desk I have left 300 rubles. As for repairing, it was just like how it was when you were younger." "Gramps")
    (add `/Game/UI/LetterSystem/BPW_ResLetter.ThisLetterClosed` _output_get (delegate `UI`))
    (else
      (`self.UI`))))

(event `SpawnTrans`
  (goto _label))

(event `UI`
  (bind _instance (`/Game/DataTypes/General/SaveAccess.Get Instance` self))
  (bind _save_game (`/Game/Blueprints/Instance.GetCurrentAutosave` _instance))
  (bind _returnvalue (`|CreateWidget` "/Game/UI/LetterSystem/Letters.Letters_C"))
  (bind _output_get (set `self.LettersUI` _returnvalue))
  (add `/Game/UI/LetterSystem/Letters.CloseLetters` _output_get (delegate `LoadSong`))
  (`UserWidget.AddToPlayerScreen` _output_get 0))

(event `AddManagement`
  (`/Game/DataTypes/General/TransitionManager.SpawnManagement` (`self.TransManage`)))

(event `LoadSong`
  (`Widget.RemoveFromParent` (`self.LettersUI`))
  (`KismetSystemLibrary.CollectGarbage`)
  (bind _returnvalue (`|CreateWidget` "/Game/UI/SongSelect.SongSelect_C"))
  (bind _output_get (set `self.SongSelectUI` _returnvalue))
  (`UserWidget.AddToPlayerScreen` _output_get 0)
  (add `/Game/UI/SongSelect.ChoiceMade` _output_get (delegate `KillSongUI`)))

(event `KillSongUI`
  (`Widget.RemoveFromParent` (`self.SongSelectUI`))
  (`KismetSystemLibrary.CollectGarbage`)
  (`self.AddManagement`))

(fn `ChangeTimeLighting`)

(fn `ChangeTimeUI`)

(fn `HideAll`
  (`Widget.SetVisibility` (`self.DayTrackUI`) "HitTestInvisible")
  (`Widget.SetVisibility` (`self.DialogueWidg`) "HitTestInvisible")
  (`Widget.SetVisibility` (`self.SongSelectUI`) "HitTestInvisible")
  (`Widget.SetVisibility` (`self.LettersUI`) "HitTestInvisible"))

(fn `PickRandomEvent`
  (params (EventPool :type "Array of /Game/DataTypes/Events/BPS_Dialogue Structure"))
  (set `self.DialogueThisScene` (`|GetArrayItem` EventPool (`KismetMathLibrary.RandomInteger` (`KismetArrayLibrary.Array_Length` EventPool)))))

(fn `SetDialogue`
  (params (DialogueInt :type Integer))
  (locals (DialogueIterator :type Integer))
  (bind _dialoguewidg (`self.DialogueWidg`))
  (bind _dialoguethisscene (`self.DialogueThisScene`))
  (bind _dialoguethisscene_2 (`self.DialogueThisScene`))
  (bind (_dialoguethisscene_eventstoapprove _dialoguethisscene_eventstokill _dialoguethisscene_letterstounlock _dialoguethisscene_dependencycount _dialoguethisscene_name _dialoguethisscene_periodofday _dialoguethisscene_dialogue _dialoguethisscene_ischoice _dialoguethisscene_choices) (break `/Game/DataTypes/Events/BPS_Dialogue` (`self.DialogueThisScene`)))
  (bind _dialoguewidg_2 (`self.DialogueWidg`))
  (bind _returnvalue (`KismetArrayLibrary.Array_Length` (break `/Game/UI/Dialogue/Dialogues` (`.Dialogue_29_3298C4F9485B3234EC9E0891EEE016FD` (break `/Game/DataTypes/Events/BPS_Dialogue` _dialoguethisscene)))))
  (bind _output_choiceshow (break `/Game/DataTypes/Events/Choice` (`|GetArrayItem` _dialoguethisscene_choices)))
  (bind (_output_speaker _output_line) (break `/Game/UI/Dialogue/LinesOfDialogue` (`|GetArrayItem` (break `/Game/UI/Dialogue/Dialogues` (`.Dialogue_29_3298C4F9485B3234EC9E0891EEE016FD` (break `/Game/DataTypes/Events/BPS_Dialogue` _dialoguethisscene_2))) (`local.DialogueIterator`))))
  (bind _output_choiceshow_2 (break `/Game/DataTypes/Events/Choice` (`|GetArrayItem` _dialoguethisscene_choices 1)))
  ;[1 1 1] Set text
  (set `local.DialogueIterator` DialogueInt)
  (`KismetSystemLibrary.PrintString` (`KismetStringLibrary.Conv_NameToString` (`.Name_39_9230A0A441BAD9099F8928974F2F1BDA` (break `/Game/DataTypes/Events/BPS_Dialogue` _dialoguethisscene_2))))
  (set `TextBlock.Text` _output_line (`/Game/UI/Dialogue/Dialogue.Passage` _dialoguewidg))
  (set `TextBlock.Text` (`KismetTextLibrary.Conv_StringToText` (`|GetEnumeratorNameAsString` _output_speaker)) (`/Game/UI/Dialogue/Dialogue.Name` _dialoguewidg))
  ;[1 1 1] End Checks
  ;;[1 1 1] If over
  (if (== _returnvalue (`local.DialogueIterator`))
    ;;[1 1 1] Kill
    (`/Game/DataTypes/General/SG_Game.ResolveDialogue` (`/Game/Blueprints/Instance.CurrentAutosave` (`self.Instance`)) (`self.DialogueThisScene`))
    (`Widget.RemoveFromParent` (`self.DialogueWidg`))
    (`KismetSystemLibrary.CollectGarbage`)
    (`KismetSystemLibrary.PrintString` "Dialogue Done")
    (`KismetSystemLibrary.PrintString` (`KismetStringLibrary.Conv_NameToString` (`.Name_39_9230A0A441BAD9099F8928974F2F1BDA` (break `/Game/DataTypes/Events/BPS_Dialogue` _dialoguethisscene))))
    (`self.DialogueOver`)
    (else
      ;;[1 1 1] If right before end
      (if (== (`local.DialogueIterator`) (- _returnvalue 1))
        ;;[1 1 1] Choices
        ;;;[1 1 1] If Is Choice
        (if _dialoguethisscene_ischoice
          (set `Widget.Visibility` "Visible" (`/Game/UI/Dialogue/Dialogue.Choice1` _dialoguewidg_2))
          (set `Widget.Visibility` "Visible" (`/Game/UI/Dialogue/Dialogue.Choice2` _dialoguewidg_2))
          (set `TextBlock.Text` _output_choiceshow (`/Game/UI/Dialogue/Dialogue.Choice1Text` _dialoguewidg_2))
          (set `TextBlock.Text` _output_choiceshow_2 (`/Game/UI/Dialogue/Dialogue.Choice2Text` _dialoguewidg_2))
          (`Widget.SetVisibility` (`/Game/UI/Dialogue/Dialogue.Continue` _dialoguewidg_2) "Hidden"))))))

(fn `ShowAll`
  (`Widget.SetVisibility` (`self.DayTrackUI`) "Visible")
  (`Widget.SetVisibility` (`self.DialogueWidg`) "Visible")
  (`Widget.SetVisibility` (`self.SongSelectUI`) "Visible")
  (`Widget.SetVisibility` (`self.LettersUI`) "Visible"))

(fn `UserConstructionScript`)