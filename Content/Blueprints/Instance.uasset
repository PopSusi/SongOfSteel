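; Game instance that runs the day-period clock, save slots and period-based event pool, using an SG_Game autosave as shared state.
; AdvanceTime steps or sets the period, blocking Morning, Afternoon and Night unless forced, then autosaves and signals time or day updates.
; EventInitialize filters saved events by period and current scene, sorts them into three priority lists and broadcasts them.
; HardSave copies the autosave to PRIMARY; R debug-skips time.
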(event Custom|RefreshSave_Event
  (CallFunction|EventInitialize)
  (Development|PrintString "refresh"))

(event Input|KeyboardEvents|DebugKeyR
  (params (Key :type Key%20Structure :default "None") (ActionValue :type Input%20Action%20Value%20Structure))
  (:Pressed
    (CallFunction|AdvanceTime true "NewEnumerator0" false)
    (CallFunction|EventInitialize)))

(fn HardSave
  (bind _save (CallFunction|GetSave "AUTOSAVE"))
  (SaveGame|SaveGametoSlot _save "PRIMARY"))

(fn InitializeGame
  (bind _save (CallFunction|GetSave "AUTOSAVE"))
  (bind _output_get (Variables|Default|SetCurrentAutosave _save))
  (EventDispatchers|BindEventtoAutosaveOccured _output_get (EventDispatchers|CreateEvent :!event Custom|RefreshSave_Event))
  (return))

(fn AdvanceTime
  (params (Force :type Boolean) (ToSkipTo :type Period%20Enum :default "NewEnumerator0") (UseEnum :type Boolean))
  (bind _currentautosave (Variables|Default|GetCurrentAutosave))
  (if UseEnum
    ;[1 1 1] Using Enum
    (Development|PrintString "Used enum to swap")
    (bind _new_day (Default|SetPeriodto (Variables|Default|GetCurrentAutosave) ToSkipTo))
    (CallFunction|Autosave)
    (CallFunction|InitializeData)
    (if true
      (Default|CallDayUpdated)
      (else
        (Default|CallTimeUpdated)))
    (Development|PrintString (Utilities|String|Append "Skipped to" (Utilities|String|EnumtoString (Variables|/Game/DataTypes/General/SG_Game.SG_Game_C|GetCurrentPeriod _currentautosave)) "New Day: " (Utilities|String|ToString(Boolean) _new_day)))
    (else
      ;[1 1 1] Is it naturally skipable?
      (switch Utilities|FlowControl|Switch|SwitchonPeriod (Variables|Default|GetCurrentPeriod)
        (:NewEnumerator0
          _)
        (:NewEnumerator1
          ;[1 1 1] Force Check
          (if Force :!label _label
            _
            (else
              ;[1 1 1] Can't Skip
              (Development|PrintString "Couldnt skip")
              (return false))))
        (:NewEnumerator2
          _)
        (:NewEnumerator3
          (goto _label))
        (:NewEnumerator4
          (goto _label))
        (:NewEnumerator5
          _))
      ;[1 1 1] Skip Period by One
      (bind _new_day_2 (Default|StepPeriod _currentautosave))
      (CallFunction|Autosave)
      (CallFunction|InitializeData)
      (if _new_day_2
        (Default|CallDayUpdated)
        (else
          (Default|CallTimeUpdated)))
      (Development|PrintString (Utilities|String|Append "Skipped to" (Utilities|String|EnumtoString (Variables|/Game/DataTypes/General/SG_Game.SG_Game_C|GetCurrentPeriod _currentautosave)) "New Day: " (Utilities|String|ToString(Boolean) _new_day_2))))))

(fn EventInitialize
  (bind _currentperiod (Variables|Default|GetCurrentPeriod))
  (bind _periood_events (CallFunction|EventsbyPeriod _currentperiod))
  (if (Utilities|Array|IsNotEmpty _periood_events)
    (bind _period_scene_events (CallFunction|EventsbyScene _periood_events))
    (if (Utilities|Array|IsNotEmpty _period_scene_events)
      (CallFunction|PrioritySort _period_scene_events)
      (Development|PrintString (Utilities|String|Append "Event possible at: " (Utilities|String|EnumtoString _currentperiod)))
      (Default|CallEventsInitialized)
      (else
        (Development|PrintString "Scene has no events")))
    (else
      (Development|PrintString "This Period is Empty"))))

(fn CheckifPeriodIsEmpty
  (bind _output_get (Variables|Default|SetCurrentPeriod (Variables|/Game/DataTypes/General/SG_Game.SG_Game_C|GetCurrentPeriod (Variables|Default|GetCurrentAutosave))))
  (bind _periood_events (CallFunction|EventsbyPeriod _output_get))
  (return (Utilities|Array|IsEmpty _periood_events)))

(fn PrioritySort
  (params (Period-Scene%20Events :type Array%20of%20BPS%20Dialogue%20Structures))
  (Utilities|Array|Clear (Variables|Default|GetLowPriorityEvents))
  (Utilities|Array|Clear (Variables|Default|GetMidPriorityEvents))
  (Utilities|Array|Clear (Variables|Default|GetHighPriorityEvents))
  (for _array_element Period-Scene%20Events
    (switch int (.Priority (Utilities|Struct|BreakBPS_Dialogue _array_element))
      (:0
        (Utilities|Array|AddUnique (Variables|Default|GetLowPriorityEvents) _array_element))
      (:1
        (Utilities|Array|AddUnique (Variables|Default|GetMidPriorityEvents) _array_element))
      (:2
        (Utilities|Array|AddUnique (Variables|Default|GetHighPriorityEvents) _array_element)))))

(fn EventsbyPeriod
  (params (PeriodOfDay :type Period%20Enum :default "NewEnumerator0"))
  (Utilities|Array|Clear (LocalVariables|GetPeriodEvents))
  (bind _values (Utilities|Map|Values (Variables|/Game/DataTypes/General/SG_Game.SG_Game_C|GetEventsPossible (Variables|Default|GetCurrentAutosave))))
  (for _array_element _values
    (bind _output_get (Variables|Default|SetTempEvent _array_element))
    (bind _array_element_2 (Utilities|Array|ForEachLoopwithBreak (.periodofday _output_get) :!label _label)
      (:LoopBody
        (if (Utilities|Enum|Equal(Enum) PeriodOfDay _array_element_2)
          (Utilities|Array|Add (LocalVariables|GetPeriodEvents) (Variables|Default|GetTempEvent))
          (goto _label Break)))
      (:Completed
        (return (LocalVariables|GetPeriodEvents))))))

(fn DayInitialize)

(fn Autosave
  (SaveGame|SaveGametoSlot (Variables|Default|GetCurrentAutosave) "AUTOSAVE"))

(fn InitializeData
  (bind _currentautosave (Variables|Default|GetCurrentAutosave))
  (Variables|Default|SetCurrentDay (Variables|/Game/DataTypes/General/SG_Game.SG_Game_C|GetCurrentDay _currentautosave))
  (Variables|Default|SetCurrentPeriod (Variables|/Game/DataTypes/General/SG_Game.SG_Game_C|GetCurrentPeriod _currentautosave)))

(fn EventsbyScene
  (params (Period%20Events :type Array%20of%20BPS%20Dialogue%20Structures))
  (for _array_element Period%20Events
    (bind _array_element_2 (Utilities|Array|ForEachLoopwithBreak (.PotentialScenes (Utilities|Struct|BreakBPS_Dialogue _array_element)) :!label _label)
      (:LoopBody
        (if (Utilities|Enum|Equal(Enum) _array_element_2 (Variables|Default|GetCurrentScene))
          (Utilities|Array|Add (LocalVariables|GetPeriodSceneEventPool) _array_element)
          (goto _label Break)))))
  (return (LocalVariables|GetPeriodSceneEventPool)))

(fn GetCurrentAutosave
  (Utilities|IsValid (Variables|Default|GetCurrentAutosave)
    (:Is%20Valid
      _)
    (:Is%20Not%20Valid
      (bind _returnvalue (SaveGame|LoadGamefromSlot "AUTOSAVE"))
      (bind _assg_game (Utilities|Casting|CastToSG_Game _returnvalue))
      (Variables|Default|SetCurrentAutosave _assg_game)))
  (return (Variables|Default|GetCurrentAutosave)))

(fn GetPuppets
  (return (Variables|/Game/DataTypes/General/SG_Game.SG_Game_C|GetPuppets (Variables|Default|GetCurrentAutosave))))